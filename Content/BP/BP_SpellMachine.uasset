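; BP_SpellMachine is a spell machine actor with constantly spinning mechanical parts.
; Every Tick it calls custom events that apply fixed local rotation steps to the bar (barre) and three gear (rouage) components.
; The bar and one gear turn together, while the other two gears have their own events, with differing directions and speeds.
; The steps are not scaled by delta time, so spin speed follows frame rate.
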(event Custom|Rotation_Rouage_1
  (Transformation|AddLocalRotation (Variables|Default|GetSpellMachine_Rouage_1_Low) "-1.300000,0.000000,0.000000" false false))

(event Custom|Rotation_Rouage_2
  (Transformation|AddLocalRotation (Variables|Default|GetSpellMachine_Rouage_2_Low) "2.000000,0.000000,0.000000" false false))

(event Custom|Rotation%20Barre
  (Transformation|AddLocalRotation (Variables|Default|GetSpellMachine_Barre_Low) "-2.000000,0.000000,0.000000" false false))

(event EventBeginPlay)

(event Collision|EventActorBeginOverlap
  (params (OtherActor :type Actor%20Object%20Reference)))

(event EventTick
  (params (DeltaSeconds :type Float%20%28single-precision%29))
  (CallFunction|RotationRouage2)
  (CallFunction|RotationRouage1)
  (CallFunction|RotationBarre))

(fn ConstructionScript)